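; BP_InventorySceneRenderer is a capture rig that renders a child actor in isolation, apparently as an inventory preview for the modular weapon system.
; The construction script stores references to the scene capture and child actor components.
; On BeginPlay, the SceneCaptureComponent2D is limited to showing only the child actor's components, including those of its own child actors.
; A yaw-spin of the child actor exists but is disconnected, so Tick does nothing.
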(event `self.ReceiveBeginPlay`
  (`SceneCaptureComponent.ShowOnlyActorComponents` (`self.SceneCaptureComponent2D`) (`ChildActorComponent.ChildActor` (`self.BP_Actor`)) true))

(event `self.ReceiveTick`
  (params (DeltaSeconds :type "Float (single-precision)")))

(fn `UserConstructionScript`
  (set `self.SceneCaptureComponent2D` (`self.SceneCaptureComponent2D`))
  (set `self.ChildComponent` (`self.BP_Actor`)))