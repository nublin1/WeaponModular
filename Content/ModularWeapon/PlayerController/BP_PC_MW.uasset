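; Player controller for the modular weapon screen, showing the main layout widget in UI-only input mode with a visible cursor.
; On local BeginPlay it pairs each inventory scene renderer with a slot widget by index, assigning its capture component and binding mouse move and wheel events.
; Existing part widgets link to weapon markers by matching part type; otherwise widgets are created from the markers.
; Tick prints the mouse position for debugging.
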(event `SighUpUI`
  (`WidgetBlueprintLibrary.SetInputMode_UIOnlyEx` self null "LockOnCapture")
  (set `self.bShowMouseCursor` true)
  (bind _returnvalue (`|CreateWidget` "/Game/ModularWeapon/UI/Layouts/WBP_MainLayout.WBP_MainLayout_C"))
  (bind _output_get (set `self.MainHUDContainer` _returnvalue))
  (`UserWidget.AddToViewport` _output_get 0)
  (`KismetSystemLibrary.Delay` 0.2)
  (for _array_element (`WeaponLayout.UInventoryItemSlotsWidgets` (`MainLayout.WeaponLayout` _output_get))
    (`InventoryItemSlotWidget.CalculateItemSlotPositions` _array_element)))

(event `self.ReceiveBeginPlay`
  (if (`self.IsLocalController`)
    (`self.SighUpUI`)
    (`KismetSystemLibrary.Delay` 0.25)
    (bind _outactors (`GameplayStatics.GetAllActorsOfClass` "/Game/ModularWeapon/BP_InventorySceneRenderer.BP_InventorySceneRenderer_C"))
    (if (> (`KismetArrayLibrary.Array_Length` _outactors) 0)
      (for (_array_element _array_index) _outactors
        (bind _output (`|GetArrayItem` (`WeaponLayout.UInventoryItemSlotsWidgets` (`MainLayout.WeaponLayout` (`self.MainHUDContainer`))) _array_index))
        (set `InventoryItemSlotWidget.CaptureComponent` (`InventorySceneRenderer.CaptureComponent` _array_element) _output)
        (add `InventoryItemSlotWidget.OnMouseMoveDelta` _output (`|CreateDelegate` _array_element :!event `RotateObject`))
        (add `InventoryItemSlotWidget.OnMouseWheelDelta` _output (`|CreateDelegate` _array_element :!event `ZoomObject`))
        (bind _partwidgets (`InventoryItemSlotWidget.PartWidgets` _output))
        (if (`KismetArrayLibrary.Array_IsNotEmpty` _partwidgets)
          (`InventoryItemSlotWidget.InitializeWidgetPositions` _output)
          (for _array_element_2 _partwidgets
            (bind _weaponmarkers (`Weapon.WeaponMarkers` (cast `Weapon` (`ChildActorComponent.ChildActor` (`InventorySceneRenderer.ChildComponent` _array_element)) :!pure true)))
            (for _array_element_3 _weaponmarkers
              (bind _returnvalue (`WeaponPartDataUtilities.AreWeaponPartPropertiesEqual` (`ItemPartWidget.WidgetTable` _array_element_2) (`ItemPartWidget.WidgetWeaponPartType` _array_element_2) (`SC_WeaponPartAttachmentPoint.WeaponPointType` _array_element_3)))
              (if _returnvalue
                (set `ItemPartWidget.TargetMarkerLinked` _array_element_3 _array_element_2)
                (set `ItemPartWidget.BrushTexture` (`SC_WeaponPartAttachmentPoint.BrushTexture` _array_element_3) _array_element_2)
                (`ItemPartWidget.UpdateVisual` _array_element_2))))
          (`InventoryItemSlotWidget.RecalculateLinesToDraw` _output)
          (else
            (for _array_element_4 _weaponmarkers
              (`InventoryItemSlotWidget.AddItemPartWidget` _output _array_element_4))))))))

(event `self.ReceiveTick`
  (params (DeltaSeconds :type "Float (single-precision)"))
  (bind (_locationx _locationy) (`WidgetLayoutLibrary.GetMousePositionScaledByDPI` self))
  (`WidgetLayoutLibrary.GetMousePositionOnViewport`)
  (`KismetSystemLibrary.PrintString` (`KismetStringLibrary.Conv_Vector2dToString` (`KismetMathLibrary.MakeVector2D` _locationx _locationy)) true false (struct :`R` 1.0 :`G` 0.903987 :`A` 1.0) 0.0))

(fn `UserConstructionScript`)