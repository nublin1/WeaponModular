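; Player controller for a modular weapon system that sets up the weapon inventory UI for the local player.
; On BeginPlay it creates the main layout in UI-only input, runs ProcessWeaponTable, then after a short delay links each scene renderer to its inventory slot widget.
; It matches or creates part widgets for each weapon's attachment markers, binds mouse and mesh-update events, and optionally centers the previewed weapon.
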(event `SighUpUI`
  (`WidgetBlueprintLibrary.SetInputMode_UIOnlyEx` self null "LockOnCapture")
  (set `self.bShowMouseCursor` true)
  (bind _returnvalue (`|CreateWidget` "/Game/ModularWeapon/UI/Layouts/WBP_MainLayout.WBP_MainLayout_C"))
  (bind _output_get (set `self.MainHUDContainer` _returnvalue))
  (`UserWidget.AddToViewport` _output_get 0))

(event `self.ReceiveBeginPlay`
  (bind _inventoryscenerendererlist (`self.InventorySceneRendererList`))
  (if (`self.IsLocalController`)
    (`self.SighUpUI`)
    (`KismetSystemLibrary.Delay` 0.04)
    (`self.ProcessWeaponTable`)
    (`KismetSystemLibrary.Delay` 0.5)
    (if (`KismetArrayLibrary.Array_IsNotEmpty` _inventoryscenerendererlist)
      (`Widget.SetVisibility` (`PanelWidget.GetChildAt` (`WeaponLayout.ContentPanel` (`MainLayout.WeaponLayout` (`self.MainHUDContainer`))) 0) "Visible")
      (for (_array_element _array_index) _inventoryscenerendererlist
        (bind _output (`|GetArrayItem` (`WeaponLayout.UInventoryItemSlotsWidgets` (`MainLayout.WeaponLayout` (`self.MainHUDContainer`))) _array_index))
        (set `InventoryItemSlotWidget.LinkedSceneRenderer` _array_element _output)
        (add `InventoryItemSlotWidget.OnMouseMoveDelta` _output (`|CreateDelegate` _array_element :!event `RotateObject`))
        (add `InventoryItemSlotWidget.OnMouseWheelDelta` _output (`|CreateDelegate` _array_element :!event `ZoomObject`))
        (bind _partwidgets (`InventoryItemSlotWidget.PartWidgets` _output))
        (if (`KismetArrayLibrary.Array_IsNotEmpty` _partwidgets)
          (`InventoryItemSlotWidget.InitializeWidgetPositions` _output)
          (for _array_element_2 _partwidgets
            (bind _weaponmarkers (`Weapon.WeaponMarkers` (cast `Weapon` (`ChildActorComponent.ChildActor` (`InventorySceneRenderer.ChildComponent` _array_element)) :!pure true)))
            (for _array_element_3 _weaponmarkers
              (`InventoryItemSlotWidget.ComparisonAndUpdateItemPartWidget` _output _array_element_2 _array_element_3)
              (add `SC_WeaponPartAttachmentPoint.OnStaticMeshUpdated` _array_element_3 (`|CreateDelegate` _array_element :!event `CenterChildComponent`))
              (if (`.bCenterWeapon` (break `CameraSettings` (`self.CameraSettings`))) :!label _label
                (`InventorySceneRenderer.CenterChildComponent` _array_element))))
          (`InventoryItemSlotWidget.RecalculateLinesToDraw` _output)
          (elif (`KismetArrayLibrary.Array_IsNotEmpty` _weaponmarkers)
            (for _array_element_4 _weaponmarkers
              (`InventoryItemSlotWidget.AddItemPartWidget` _output _array_element_4)
              (add `SC_WeaponPartAttachmentPoint.OnStaticMeshUpdated` _array_element_4 (`|CreateDelegate` _array_element :!event `CenterChildComponent`))
              (goto _label))))))))

(event `self.ReceiveTick`
  (params (DeltaSeconds :type "Float (single-precision)")))

(fn `UserConstructionScript`)